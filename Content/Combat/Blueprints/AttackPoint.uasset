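; Combat attack point component that tracks its own motion and uses it as the direction of hits on Goons.
; Each tick it derives velocity from the change in world location.
; Hit projects that velocity onto a horizontal plane based at the Goon's location, normalizes it, passes it to ApplyHit and draws a debug arrow.
; Whiff draws a debug arrow along the velocity, pointing up when nearly still.
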(event `self.ReceiveBeginPlay`
  (set `self.OldLocation` (`self.K2_GetComponentLocation`)))

(event `self.ReceiveTick`
  (params (DeltaSeconds :type "Float (single-precision)"))
  (`self.UpdateVelocity` DeltaSeconds))

(fn `Draw Debug`
  (params (Duration :type "Float (double-precision)"))
  (locals (ArrowDirection :type "Vector Structure" :default (0.0 0.0 0.0)) (Speed :type "Float (double-precision)" :default 0.0) (ArrowEnd :type "Vector Structure" :default (0.0 0.0 0.0)) (CachedDuration :type "Float (double-precision)"))
  (bind _velocity (`self.Velocity`))
  (bind _returnvalue (`KismetMathLibrary.VSize` _velocity))
  (set `local.CachedDuration` Duration)
  (set `local.Speed` _returnvalue)
  (set `local.ArrowDirection` (`KismetMathLibrary.SelectVector` (`KismetMathLibrary.Normal` _velocity) (0.0 0.0 1.0) (> _returnvalue 0.1)))
  (set `local.ArrowEnd` (+ (`self.K2_GetComponentLocation`) (* (`local.ArrowDirection`) 50.0)))
  (`KismetSystemLibrary.DrawDebugArrow` (`self.K2_GetComponentLocation`) (`local.ArrowEnd`) 20.0 (struct :`R` 1.0 :`G` 1.0 :`A` 1.0) (`local.CachedDuration`) 2.0))

(fn `GetVelocity`
  (returns (Velocity :type "Vector Structure"))
  (return (`self.Velocity`)))

(fn `Hit`
  (params (Goon :type "/Game/Characters/Goon/Blueprints/GoonCharacterBP Object Reference"))
  (bind _returnvalue (`Actor.K2_GetActorLocation` Goon))
  (bind _returnvalue_2 (`KismetMathLibrary.Normal` (`KismetMathLibrary.ProjectPointOnToPlane` (`self.Velocity`) _returnvalue (0.0 0.0 1.0))))
  (`/Game/Characters/Goon/Blueprints/GoonCharacterBP.Apply Hit` Goon _returnvalue_2)
  (`KismetSystemLibrary.DrawDebugArrow` _returnvalue (+ (* _returnvalue_2 100.0) _returnvalue) 20.0 (struct :`R` 1.0 :`G` 1.0 :`A` 1.0) 1.0 2.0))

(fn `UpdateVelocity`
  (params (Delta :type "Float (double-precision)"))
  (set `self.Velocity` (/ (- (`self.K2_GetComponentLocation`) (`self.OldLocation`)) Delta))
  (set `self.OldLocation` (`self.K2_GetComponentLocation`)))

(fn `Whiff`
  (`self.Draw Debug` 1.0))