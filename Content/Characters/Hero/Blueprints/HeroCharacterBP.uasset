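; Player hero character Blueprint that handles melee hit detection, jump state and blink visual direction, and registers with the game mode's CombatManager.
; Construction maps AttackPoint components by point and sets the light combo to the blink combo.
; NotifyAttack line-traces forward, calling Hit on the selected point for goons, otherwise Whiff.
; Tick feeds BlinkDirection to a material parameter collection, using actor forward during montages, otherwise the last blink direction.
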(event `self.OnJumped`
  (set `self.IsJumping` true))

(event `self.OnLanded`
  (params (Hit :type "HitResult Structure (by ref)"))
  (set `self.IsJumping` false))

(event `self.ReceiveTick`
  (params (DeltaSeconds :type "Float (single-precision)"))
  (bind _returnvalue (`self.GetCurrentMontage`))
  (`/Engine/EditorBlueprintResources/StandardMacros.IsValid` _returnvalue
    (:`Is Valid`
      (`KismetMaterialLibrary.SetVectorParameterValue` "/Game/Characters/Hero/HeroMatCollection.HeroMatCollection" "BlinkDirection" (`KismetMathLibrary.Conv_VectorToLinearColor` (`self.GetActorForwardVector`))))
    (:`Is Not Valid`
      (`KismetMaterialLibrary.SetVectorParameterValue` "/Game/Characters/Hero/HeroMatCollection.HeroMatCollection" "BlinkDirection" (`KismetMathLibrary.Conv_VectorToLinearColor` (`BlinkComponent.LastBlinkDirection` (`self.BlinkComponent`)))))))

(event `self.ReceiveBeginPlay`
  (bind _returnvalue (`self.GetComponentByClass` (`GameplayStatics.GetGameMode`) "/Script/BlinkGame.CombatManager"))
  (`/Engine/EditorBlueprintResources/StandardMacros.IsValid` _returnvalue
    (:`Is Valid`
      (`CombatManager.RegisterPlayer` _returnvalue self))))

(fn `NotifyAttack`
  (params (PointSource :type "EAttackPointEnum Enum" :default "None"))
  (locals (AttackPoint :type "/Game/Combat/Blueprints/AttackPoint Object Reference") (HitTestVector :type "Vector Structure" :default (0.0 0.0 0.0)))
  (bind _returnvalue (`self.K2_GetActorLocation`))
  (bind (_value _returnvalue_2) (`BlueprintMapLibrary.Map_Find` (`self.AttackPoints`) PointSource))
  (bind _returnvalue_3 (+ _returnvalue (`local.HitTestVector`)))
  (if _returnvalue_2
    (set `local.AttackPoint` _value)
    (set `local.HitTestVector` (* (`self.GetActorForwardVector`) (`self.HitRange`)))
    (bind (_outhit _returnvalue_4) (`KismetSystemLibrary.LineTraceSingle` _returnvalue _returnvalue_3 "TraceTypeQuery1"))
    (if _returnvalue_4
      (bind _asgoon_character_bp (cast `/Game/Characters/Goon/Blueprints/GoonCharacterBP` (`.HitActor` (`GameplayStatics.BreakHitResult` _outhit)))
        (:`then`
          (`/Game/Combat/Blueprints/AttackPoint.Hit` (`local.AttackPoint`) _asgoon_character_bp))
        (:`CastFailed`
          (`/Game/Combat/Blueprints/AttackPoint.Whiff` (`local.AttackPoint`))))
      (else
        (`DrawDebugLibrary.DrawArrow` (`DrawDebugLibrary.GetWorldFromActor` self) _returnvalue _returnvalue_3 20.0 (struct :`R` 1.0 :`A` 1.0) 1.0)
        (`/Game/Combat/Blueprints/AttackPoint.Whiff` (`local.AttackPoint`))))))

(fn `UserConstructionScript`
  (set `self.LightAttackCombo` (`self.BlinkAttackCombo`))
  (for _array_element (`self.K2_GetComponentsByClass` "/Game/Combat/Blueprints/AttackPoint.AttackPoint_C")
    (`BlueprintMapLibrary.Map_Add` (`self.AttackPoints`) (`/Game/Combat/Blueprints/AttackPoint.Point` _array_element) _array_element)))