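; BlinkAttackCombo is a component that plays a character's attack montage as a sequence of combo sections.
; It caches its owning Character on BeginPlay.
; Each Play call starts the montage at the current named section and advances the index, wrapping to the first when out of range.
; SetSection can set an override index that, when non-negative, replaces the cycled section while the counter keeps advancing.
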(event `self.ReceiveBeginPlay`
  (bind _ascharacter (cast `Character` (`self.GetOwner`)))
  (set `self.Character` _ascharacter))

(event `SetSection`
  (params (NewSectionOverride :type Integer))
  (if (< NewSectionOverride (`KismetArrayLibrary.Array_Length` (`self.SectionNames`)))
    (set `self.SectionOverride` NewSectionOverride)))

(event `ComboInterface.Play`
  (bind _sectionoverride (`self.SectionOverride`))
  (`/Engine/EditorBlueprintResources/StandardMacros.IsValid` (`self.Character`)
    (:`Is Valid`
      (if (not (`KismetMathLibrary.InRange_IntInt` (`self.CurrentSection`) 0 (`KismetArrayLibrary.Array_Length` (`self.SectionNames`)) true false))
        (set `self.CurrentSection` 0))
      (`Character.PlayAnimMontage` (`self.Character`) (`self.Montage`) 1.0 (`|GetArrayItem` (`self.SectionNames`) (`KismetMathLibrary.SelectInt` (`self.CurrentSection`) _sectionoverride (< _sectionoverride 0))))
      (`/Engine/EditorBlueprintResources/StandardMacros.IncrementInt` (`self.CurrentSection`)))))